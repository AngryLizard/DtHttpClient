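; BP_DTGameController is a player controller for a cursor-driven game that converts the mouse position into a world location.
; On BeginPlay it shows the cursor, disables viewport mouse capture and switches input to UI only.
; QueryMousePosition deprojects the cursor, sphere-traces along that ray on the Visibility channel up to HitDistance, and passes any hit location to CallOnPositionClicked.
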(event Custom|QueryMousePosition
  (bind (_worldlocation _worlddirection _returnvalue) (Game|Player|ConvertMouseLocationToWorldSpace))
  (if _returnvalue
    (bind (_outhit _returnvalue_2) (Collision|SphereTraceByChannel _worldlocation (+ _worldlocation (* _worlddirection (Variables|Default|GetHitDistance))) 1e+01 "TraceTypeQuery1" false 0 "None"))
    (if _returnvalue_2
      (Default|CallOnPositionClicked (.Location (Collision|BreakHitResult _outhit))))))

(event EventBeginPlay
  (Variables|Default|SetbShowMouseCursor true)
  (Class|GameplayStatics|SetViewportMouseCaptureMode "NoCapture")
  (Input|SetInputModeUIOnly self 0 "DoNotLock" false))

(fn ConstructionScript)